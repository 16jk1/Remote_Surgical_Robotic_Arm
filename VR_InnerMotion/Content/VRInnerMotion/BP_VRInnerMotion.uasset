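; BP_VRInnerMotion is a VR pawn that moves and turns when the player's virtual hands touch control orbs.
; Each tick, either hand overlapping the rotate orbs adds yaw input, while the forward orb adds movement along the actor's forward vector.
; Overlapped orbs swap material as feedback.
; HMD orientation and position reset on BeginPlay and Left X press, and touch inputs switch hand animations between open and can-grab.
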(event EventBeginPlay
  ;[1 0.1935 0.6712] Reset View Position
  (Class|HeadMountedDisplayFunctionLibrary|ResetOrientationandPosition 0.0 "OrientationAndPosition"))

(event EventTick
  (params (DeltaSeconds :type Float%20%28single-precision%29))
  (bind _handl (Variables|Default|GetHandL))
  (bind _handl_2 (Variables|Default|GetHandL))
  (bind _rotateright (Variables|Default|GetRotateRight))
  (bind _rotationspeed (Variables|Default|GetRotationSpeed))
  (bind _handr (Variables|Default|GetHandR))
  (bind _rotateright_2 (Variables|Default|GetRotateRight))
  (bind _rotateleft (Variables|Default|GetRotateLeft))
  (bind _rotateleft_2 (Variables|Default|GetRotateLeft))
  (bind _handl_3 (Variables|Default|GetHandL))
  (bind _handr_2 (Variables|Default|GetHandR))
  (bind _moveforward (Variables|Default|GetMoveForward))
  (bind _moveforward_2 (Variables|Default|GetMoveForward))
  (bind _handr_3 (Variables|Default|GetHandR))
  (bind _returnvalue (Class|PrimitiveComponent|IsOverlappingComponent _handl _rotateright))
  (bind _returnvalue_2 (Class|PrimitiveComponent|IsOverlappingComponent _handr_3 _rotateright_2))
  (bind _returnvalue_3 (Class|PrimitiveComponent|IsOverlappingComponent _handr _rotateleft_2))
  (bind _returnvalue_4 (Class|PrimitiveComponent|IsOverlappingComponent _handl_2 _rotateleft))
  (bind _returnvalue_5 (Class|PrimitiveComponent|IsOverlappingComponent _handl_3 _moveforward))
  (bind _returnvalue_6 (Class|PrimitiveComponent|IsOverlappingComponent _handr_2 _moveforward_2))
  (bind _returnvalue_7 (or _returnvalue_4 _returnvalue_3))
  (bind _returnvalue_8 (or _returnvalue_5 _returnvalue_6))
  (bind _returnvalue_9 (or _returnvalue _returnvalue_2))
  (Utilities|FlowControl|Sequence
    (:then_0
      ;[0 0.8826 0.98] Movement Controls
      (Variables|Default|SetbRotRight _returnvalue_9)
      (Variables|Default|SetbTextureR _returnvalue_9)
      (Variables|Default|SetbRotLeft _returnvalue_7)
      (Variables|Default|SetbTextureL _returnvalue_7)
      (Pawn|Input|AddControllerYawInput (+ (* (Math|Conversions|ToFloat(Boolean) (Variables|Default|GetbRotRight)) 1.0 _rotationspeed) (* (Math|Conversions|ToFloat(Boolean) (Variables|Default|GetbRotLeft)) -1.0 _rotationspeed))))
    (:then_1
      (Variables|Default|SetbMoveForward _returnvalue_8)
      (Variables|Default|SetbTextureF _returnvalue_8)
      (Pawn|Input|AddMovementInput (Transformation|GetActorForwardVector) (* (Math|Conversions|ToFloat(Boolean) (Variables|Default|GetbMoveForward)) (Variables|Default|GetMovementSpeed)) false))
    (:then_2
      ;[0.1102 0.5971 1] Orb Animation when Overlapped
      (if (Variables|Default|GetbTextureR)
        (Rendering|Material|SetMaterial (Variables|Default|GetRotateRight) 0 "/Game/VirtualReality/Materials/M_SplineArcMat.M_SplineArcMat")
        (else
          (Rendering|Material|SetMaterial (Variables|Default|GetRotateRight) 0 "/Game/VirtualReality/Materials/M_ArcEndpoint.M_ArcEndpoint"))))
    (:then_3
      (if (Variables|Default|GetbTextureL)
        (Rendering|Material|SetMaterial (Variables|Default|GetRotateLeft) 0 "/Game/VirtualReality/Materials/M_SplineArcMat.M_SplineArcMat")
        (else
          (Rendering|Material|SetMaterial (Variables|Default|GetRotateLeft) 0 "/Game/VirtualReality/Materials/M_ArcEndpoint.M_ArcEndpoint"))))
    (:then_4
      (if (Variables|Default|GetbTextureF)
        (Rendering|Material|SetMaterial (Variables|Default|GetMoveForward) 0 "/Game/VirtualReality/Materials/M_SplineArcMat.M_SplineArcMat")
        (else
          (Rendering|Material|SetMaterial (Variables|Default|GetMoveForward) 0 "/Game/VirtualReality/Materials/M_ArcEndpoint.M_ArcEndpoint"))))))

(event Input|ActionEvents|InputActionLeft_Touch
  (params (Key :type Key%20Structure :default "None"))
  ;[0.124 0.1227 1] Hand Animations
  (:Pressed
    (Components|Animation|SetAnimation (Variables|Default|GetHandL) "/Game/VirtualReality/Mannequin/Animations/MannequinHand_Right_CanGrab.MannequinHand_Right_CanGrab"))
  (:Released
    (Components|Animation|SetAnimation (Variables|Default|GetHandL) "/Game/VirtualReality/Mannequin/Animations/MannequinHand_Right_Open.MannequinHand_Right_Open")))

(event Input|ActionEvents|InputActionLeft_X_Press
  (params (Key :type Key%20Structure :default "None"))
  ;[1 0.1935 0.6712] Reset View Position
  (:Pressed
    (Class|HeadMountedDisplayFunctionLibrary|ResetOrientationandPosition 0.0 "OrientationAndPosition")))

(event Input|ActionEvents|InputActionRight_Touch
  (params (Key :type Key%20Structure :default "None"))
  ;[0.124 0.1227 1] Hand Animations
  (:Pressed
    (Components|Animation|SetAnimation (Variables|Default|GetHandR) "/Game/VirtualReality/Mannequin/Animations/MannequinHand_Right_CanGrab.MannequinHand_Right_CanGrab"))
  (:Released
    (Components|Animation|SetAnimation (Variables|Default|GetHandR) "/Game/VirtualReality/Mannequin/Animations/MannequinHand_Right_Open.MannequinHand_Right_Open")))

(fn ConstructionScript)